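; Spline-driven sidewalk actor that lays deformed mesh segments along an editable path.
; The construction script adds one spline mesh component per pair of neighboring spline points, using their local locations and tangents.
; Each segment has a negative Z scale, with start and end heights negated to compensate, while tangents pass through unchanged.
; The event graph has no active logic.
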(fn `UserConstructionScript`
  (locals (NewLocalVar_0 :type "Float (double-precision)" :default 0.0))
  (bind _spline (`self.Spline`))
  (for _index (range (+ (- (`SplineComponent.GetNumberOfSplinePoints` _spline) 2) 1))
    (bind _returnvalue (`AddComponent|NODE_AddSplineMeshComponent-0` :`RelativeTransform` (`KismetMathLibrary.MakeTransform` (0.0 0.0 0.0) (struct) (1.0 1.0 -1.0))))
    (`SceneComponent.K2_AttachToComponent` _spline (`self.DefaultSceneRoot`) "None" "KeepRelative" "KeepRelative" "KeepRelative" true)
    (bind (_location _tangent) (`SplineComponent.GetLocationAndTangentAtSplinePoint` _spline _index "Local"))
    (bind (_location_2 _tangent_2) (`SplineComponent.GetLocationAndTangentAtSplinePoint` _spline (+ _index 1) "Local"))
    (`SplineMeshComponent.SetStartAndEnd` _returnvalue (`KismetMathLibrary.MakeVector` (.x _location) (.y _location) (* (.z _location) -1.0)) _tangent (`KismetMathLibrary.MakeVector` (.x _location_2) (.y _location_2) (* (.z _location_2) -1.0)) _tangent_2 true)))